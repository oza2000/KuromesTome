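; Action-adventure character with mana-driven boost, fireball and shield abilities, plus hit sounds, ragdoll death and incoming-damage notification.
; Boost temporarily raises walk speed but leaves jump velocity raised, while left mouse spawns a fireball.
; Holding right mouse roots the character, shows a blocking sphere and zeroes Health; release resets Health to 100 and Mana to 6.
; Tick regenerates mana up to its cap and disables input while it is low.
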(event `Key|LeftShift`
  (params (Key :type "Key Structure")))

(event `Key|E`
  (params (Key :type "Key Structure"))
  (bind _charactermovement (`self.CharacterMovement`))
  (:`Pressed`
    (if (`self.Can Boost`)
      (set `self.mana` (- (`self.mana`) 3.0) :!label _label)
      (set `CharacterMovementComponent.MaxWalkSpeed` 1200.0 _charactermovement :!label _label_2)
      (set `CharacterMovementComponent.JumpZVelocity` 1200.0 (`self.CharacterMovement`))
      (`KismetSystemLibrary.Delay` 7.5)
      (set `CharacterMovementComponent.MaxWalkSpeed` 600.0 _charactermovement))))

(event `Key|LeftShift`
  (params (Key :type "Key Structure"))
  (:`Pressed`
    (if (`self.Can Boost`)
      (goto _label))))

(event `Key|LeftShift`
  (params (Key :type "Key Structure"))
  (:`Pressed`
    (if (`self.Can Boost`)
      (goto _label_2))))

(event `Key|LeftMouseButton`
  (params (Key :type "Key Structure"))
  (:`Pressed`
    (set `self.mana` (- (`self.mana`) 3.0))
    (`|SpawnActorFromClass` "/Game/NewFolder/fireball.fireball_C" (`KismetMathLibrary.MakeTransform` (`self.K2_GetActorLocation`) (`self.K2_GetActorRotation`)) "Undefined" "OverrideRootScale" null null)))

(event `self.ReceivePointDamage`
  (params (Damage :type "Float (single-precision)") (DamageType :type "DamageType Object Reference") (HitLocation :type "Vector Structure") (HitNormal :type "Vector Structure") (HitComponent :type "PrimitiveComponent Object Reference") (BoneName :type Name) (ShotFromDirection :type "Vector Structure") (InstigatedBy :type "Controller Object Reference") (DamageCauser :type "Actor Object Reference") (HitInfo :type "HitResult Structure (by ref)"))
  ;[0.1 0.1 0.1] Play a hit sound
  (`parent.ReceivePointDamage` Damage DamageType HitLocation HitNormal HitComponent BoneName ShotFromDirection InstigatedBy DamageCauser HitInfo)
  (`GameplayStatics.PlaySoundAtLocation` "/Game/AdventureKit/AK_Core/Weapons/Sounds/SC_Sword_Hit.SC_Sword_Hit" (`self.K2_GetActorLocation`)))

(event `self.ReceiveTick`
  (params (DeltaSeconds :type "Float (single-precision)"))
  (`|ExecutionSequence`
    (:`then_0`
      (if (>= (`self.mana`) 10.0)
        (set `self.mana` 10.0)
        (else
          (set `self.mana` (+ (`self.mana`) 0.05) :!label _label_3))))
    (:`then_1`
      (if (< (`self.mana`) 3.0)
        (`self.DisableInput` null)
        (else
          (`self.EnableInput` null))))))

(event `self.Died`
  (params (Killer :type "Controller Object Reference") (DamageEvent :type "DamageEvent Structure (by ref)") (HitLocation :type "Vector Structure"))
  (bind _mesh (`self.Mesh`))
  ;[0.1 0.1 0.1] Turn on ragdoll on death
  (`parent.Died` Killer DamageEvent HitLocation)
  (`PrimitiveComponent.SetSimulatePhysics` _mesh true)
  (`PrimitiveComponent.WakeAllRigidBodies` _mesh)
  (`PrimitiveComponent.SetCollisionEnabled` _mesh "QueryAndPhysics")
  (`PrimitiveComponent.SetCollisionEnabled` (`self.CapsuleComponent`) "NoCollision")
  (`PrimitiveComponent.SetCollisionResponseToAllChannels` (`self.CapsuleComponent`) "ECR_Ignore"))

(event `/Game/AdventureKit/AK_Core/Weapons/Blueprints/BPI_IncomingDamageReceiver.Notify Incoming Damage`
  (params (Instigator :type "AdvKitCharacter Object Reference") (Weapon :type "AdvKitWeapon Object Reference"))
  ;[0.1 0.1 0.1] Bind interface event to event dispatcher
  (`self.Notify Of Incoming Damage` Instigator Weapon))

(event `Key|RightMouseButton`
  (params (Key :type "Key Structure"))
  (bind _mana (`self.mana`))
  (:`Pressed`
    (if (`self.Can Shield`)
      (set `CharacterMovementComponent.MaxWalkSpeed` 0.0 (`self.CharacterMovement`))
      (set `CharacterMovementComponent.JumpZVelocity` 0.0 (`self.CharacterMovement`))
      (set `self.Health` 0.0)
      (`PrimitiveComponent.SetCollisionResponseToAllChannels` (`self.Sphere`) "ECR_Block")
      (`PrimitiveComponent.SetCollisionResponseToChannel` (`self.Sphere`) "ECC_Pawn" "ECR_Block")
      (`SceneComponent.SetVisibility` (`self.Sphere`) true false)
      (if (`KismetMathLibrary.InRange_FloatFloat` _mana 0.0 3.0)
        (set `self.mana` (- _mana 1.0))
        (if (<= _mana 0.1)
          (goto _label_3)))))
  (:`Released`
    (if (`self.Can Shield`)
      (set `CharacterMovementComponent.MaxWalkSpeed` 600.0 (`self.CharacterMovement`))
      (set `CharacterMovementComponent.JumpZVelocity` 600.0 (`self.CharacterMovement`))
      (set `self.Health` 100.0)
      (`PrimitiveComponent.SetCollisionResponseToAllChannels` (`self.Sphere`) "ECR_Ignore")
      (`SceneComponent.SetVisibility` (`self.Sphere`) false false)
      (set `self.mana` 6.0))))

(event `self.CharacterMovement.OnComponentActivated`
  (params (Component :type "ActorComponent Object Reference") (bReset :type Boolean)))

(fn `Get Target Point`
  (returns (Target :type "AdvKitTargetPoint Object Reference"))
  (return (cast `AdvKitTargetPoint` (`ChildActorComponent.ChildActor` (`self.Target`)) :!pure true)))

(fn `UserConstructionScript`
  (`parent.UserConstructionScript`))